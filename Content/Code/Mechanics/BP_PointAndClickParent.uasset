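; BP_PointAndClickParent is a base actor for point-and-click objects, with a widget that appears when Clicked is called.
; On BeginPlay it hides the widget and searches actors tagged "Clickable" for its own object name.
; On a match it sets its Name text to "Clickable" plus its one-based position in that list.
; Clicked only unhides the widget; nothing here hides it again.
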(event EventBeginPlay
  (Development|SetHiddeninGame (Variables|Default|GetWidget) true false)
  (bind _outactors (Actor|GetAllActorswithTag "Clickable"))
  (bind (_array_element _array_index) (Utilities|Array|ForEachLoopwithBreak _outactors :!label _label)
    (:LoopBody
      (if (Utilities|Enum|Equal(Enum) (Utilities|GetObjectName self) (Utilities|GetObjectName _array_element))
        (Variables|Default|SetName (Utilities|Text|ToText(String) (Utilities|String|Append "Clickable" " " (Utilities|String|ToString(Integer) (+ _array_index 1)))))
        (goto _label Break)))))

(event Collision|EventActorBeginOverlap
  (params (OtherActor :type Actor%20Object%20Reference)))

(event EventTick
  (params (DeltaSeconds :type Float%20%28single-precision%29)))

(fn ConstructionScript)

(fn Clicked
  (Development|SetHiddeninGame (Variables|Default|GetWidget) false false))